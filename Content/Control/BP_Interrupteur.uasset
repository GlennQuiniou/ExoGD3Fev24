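; BP_Interrupteur is a light switch that turns nearby fluorescent lamps on and off through a scaled trigger box.
; EventSetLight alternates between playing and reversing a timeline that drives the box's uniform world scale.
; BP_LampFluor and BP_LampFluorSmall actors have their point light zeroed on entering the box and set to a fixed intensity on leaving, so lights follow the box's changing extent.
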(event OnComponentBeginOverlap(Box)
  (params (OverlappedComponent :type Primitive%20Component%20Object%20Reference) (OtherActor :type Actor%20Object%20Reference) (OtherComp :type Primitive%20Component%20Object%20Reference) (OtherBodyIndex :type Integer) (bFromSweep :type Boolean) (SweepResult :type Hit%20Result%20Structure%20%28by%20ref%29))
  (bind _asbp_lamp_fluor_small (Utilities|Casting|CastToBP_LampFluorSmall OtherActor)
    (:then
      (Rendering|Components|Light|SetIntensity (Variables|/Game/HQ_ResidentialHouse/Actors/BP_LampFluorSmall.BP_LampFluorSmall_C|GetPointLight _asbp_lamp_fluor_small) 0.0))
    (:CastFailed
      (bind _asbp_lamp_fluor (Utilities|Casting|CastToBP_LampFluor OtherActor))
      (Rendering|Components|Light|SetIntensity (Variables|/Game/HQ_ResidentialHouse/Actors/BP_LampFluor.BP_LampFluor_C|GetPointLight _asbp_lamp_fluor) 0.0))))

(event OnComponentEndOverlap(Box)
  (params (OverlappedComponent :type Primitive%20Component%20Object%20Reference) (OtherActor :type Actor%20Object%20Reference) (OtherComp :type Primitive%20Component%20Object%20Reference) (OtherBodyIndex :type Integer))
  (bind _asbp_lamp_fluor_small (Utilities|Casting|CastToBP_LampFluorSmall OtherActor)
    (:then
      (Rendering|Components|Light|SetIntensity (Variables|/Game/HQ_ResidentialHouse/Actors/BP_LampFluorSmall.BP_LampFluorSmall_C|GetPointLight _asbp_lamp_fluor_small) 4e+02))
    (:CastFailed
      (bind _asbp_lamp_fluor (Utilities|Casting|CastToBP_LampFluor OtherActor))
      (Rendering|Components|Light|SetIntensity (Variables|/Game/HQ_ResidentialHouse/Actors/BP_LampFluor.BP_LampFluor_C|GetPointLight _asbp_lamp_fluor) 4e+02))))

(event Custom|EventSetLight
  (Utilities|FlowControl|FlipFlop
    (:A
      (bind _newtrack (Timeline|Timeline_Interrupteur PlayFromStart)
        (:Update
          (Transformation|SetWorldScale3D (Variables|Default|GetBox) (Math|Vector|MakeVector _newtrack _newtrack _newtrack)))))
    (:B
      (Timeline|Timeline_Interrupteur ReverseFromEnd))))

(event EventBeginPlay)

(event Collision|EventActorBeginOverlap
  (params (OtherActor :type Actor%20Object%20Reference)))

(event EventTick
  (params (DeltaSeconds :type Float%20%28single-precision%29)))

(fn ConstructionScript)